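; BP_GA_Item_Food is a 2D food pickup that lowers a unit's hunger once when a non-AI unit interacts with it.
; Interact updates CurrentHunger immediately, clamped at MinHunger, then queues an action named "Drink" and the item's destruction.
; AnimateAction later applies the visual side: it adjusts the food bar, hides the item and plays a placeholder potion sound.
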(event EventAnimateAction
  (params (Action :type F%20Action%20Structure))
  (bind _asbp_unit_2d (Utilities|Casting|CastToBP_Unit_2D (CallFunction|GetUnit Action)))
  (Default|ModifyFoodBar _asbp_unit_2d (* (CallFunction|GetFloat Action) -1.0))
  (Rendering|SetActorHiddenInGame true)
  ;[1 0 0] Change to food Sound
  (Audio|PlaySound2D "/Game/AdvancedTurnBasedTileToolkit/Maps/2D/Items/A_Potion.A_Potion" 1.0 1.0 0.0 0 0))

(event EventInteract
  (params (TriggeringActor :type Actor%20Object%20Reference) (InteractionType :type EInteract%20Enum :default "NewEnumerator0") (CurrentPathIndex :type Integer))
  (bind _asbp_unit (Utilities|Casting|CastToBP_Unit TriggeringActor))
  (if (not (Variables|/Game/AdvancedTurnBasedTileToolkit/Core/Units/BP_Unit.BP_Unit_C|GetbAIControlled _asbp_unit))
    (Utilities|FlowControl|DoOnce false
      (:Completed
        (bind _asbp_unit_2d (Utilities|Casting|CastToBP_Unit_2D TriggeringActor))
        (Variables|/Game/AdvancedTurnBasedTileToolkit/Maps/2D/Units/BP_Unit_2D.BP_Unit_2D_C|SetCurrentHunger _asbp_unit_2d (Math|Integer|Max(Integer) (Variables|/Game/AdvancedTurnBasedTileToolkit/Maps/2D/Units/BP_Unit_2D.BP_Unit_2D_C|GetMinHunger _asbp_unit_2d) (- (Variables|/Game/AdvancedTurnBasedTileToolkit/Maps/2D/Units/BP_Unit_2D.BP_Unit_2D_C|GetCurrentHunger _asbp_unit_2d) (Variables|Default|GetHungerSatisfyAmmount))))
        (Utilities|QueueActionSingles :Executing%20Object self :Action%20Name "Drink" :Instant%20Deactivate true :Float (Math|Conversions|ToFloat(Integer) (Variables|Default|GetHungerSatisfyAmmount)) :Unit _asbp_unit_2d)
        (Utilities|QueueDestroy (Utilities|Array|MakeArray self))))))

(fn ConstructionScript
  (|CallParentFunction))