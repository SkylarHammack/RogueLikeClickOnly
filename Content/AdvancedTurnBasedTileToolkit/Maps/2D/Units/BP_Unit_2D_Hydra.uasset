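; 2D Hydra unit for the turn-based tile toolkit that grows heads when wounded and ends the game when killed.
; Non-lethal damage raises its head count up to a cap and queues a GrowHead action.
; Animating that action waits briefly, plays a sound and swaps to the sprite matching the head count.
; On death it flags game over on the turn manager and queues the GameOver action.
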(event EventTakeDamage
  (params (Damage :type Float%20%28single-precision%29) (bAutoAnimate :type Boolean))
  (|CallParentFunction Damage bAutoAnimate)
  (if (> (Variables|Default|GetCurrentHealth) 0.0)
    (if (< (Variables|Default|GetHeads) 5)
      (bind _result (Math|Integer|IncrementInt (Variables|Default|GetHeads))
        (:%20%20
          (Utilities|QueueActionSingles self "GrowHead" "NewEnumerator0" false -1 false 0.0 false _result 0.0))))))

(event EventKillUnit
  (params (bAutoAnimate :type Boolean))
  (|CallParentFunction bAutoAnimate)
  (bind _turnmanager (Utilities|GetTurnManager))
  (Variables|/Game/AdvancedTurnBasedTileToolkit/Core/BP_TurnManager.BP_TurnManager_C|SetbGameOver _turnmanager true)
  (Utilities|QueueActionSingles :Executing%20Object _turnmanager :Action%20Name "GameOver" :Instant%20Deactivate true :Unit self))

(event EventAnimateAction
  (params (Action :type F%20Action%20Structure))
  (switch name (CallFunction|GetActionName Action)
    (:Default
      (|CallParentFunction Action))
    (:GrowHead
      (Utilities|FlowControl|Delay 0.5)
      (Audio|PlaySound2D "/Game/AdvancedTurnBasedTileToolkit/Core/Abilities/A_Discover.A_Discover" 1.0 1.0 0.0 0 0)
      (Rendering|Components|Sprite|SetSprite (Variables|Default|GetUnitSprite) (Utilities|Select :Index (CallFunction|GetInteger Action) :Option%200 "/Game/AdvancedTurnBasedTileToolkit/Maps/2D/Units/SPR_Hydra1.SPR_Hydra1" :Option%201 "/Game/AdvancedTurnBasedTileToolkit/Maps/2D/Units/SPR_Hydra1.SPR_Hydra1" :Option%202 "/Game/AdvancedTurnBasedTileToolkit/Maps/2D/Units/SPR_Hydra2.SPR_Hydra2" :Option%203 "/Game/AdvancedTurnBasedTileToolkit/Maps/2D/Units/SPR_Hydra3.SPR_Hydra3" :Option%204 "/Game/AdvancedTurnBasedTileToolkit/Maps/2D/Units/SPR_Hydra4.SPR_Hydra4" :Option%205 "/Game/AdvancedTurnBasedTileToolkit/Maps/2D/Units/SPR_Hydra5.SPR_Hydra5"))
      (Utilities|EndAction))))

(fn ConstructionScript
  (|CallParentFunction))